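; Spell casting component that manages its owner's spell list, with mana or health (blood magic) costs, cooldowns and recharging stock.
; Button release checks cost and cooldowns, then starts a Haste-scaled cast timer that movement beyond Focus tolerance cancels.
; Tick runs regeneration and timers; a finished cast pays the cost, spawns the spell actor and configures its Spell component.
; Channelling is an empty stub, and targeting decal spawns are unwired.
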(event Custom|Set%20Cast%20Timer
  (bind _spell_list (Variables|Default|GetSpell%20List))
  (bind _selected_spell (Variables|Default|GetSelected%20Spell))
  (bind _stats (Variables|Default|GetStats))
  (bind _item (Utilities|Array|Get(acopy) _spell_list _selected_spell))
  (bind _returnvalue (* (.casttime _item) (.haste (.secondary _stats))))
  ;[1 1 1] Cast Setup
  (if (.blood_magic _item)
    (if (> (Variables|Default|GetCurrent%20Life) (.mana _item))
      (if (Math|Boolean|ANDBoolean (or (<= (.current_cooldown _item) 0.0) (> (.stock_current _item) 0)) (not (Variables|Cast|GetCast)) (<= (Variables|Default|GetGlobal%20Cooldown) 0.0)) :!label _label
        (Variables|Default|SetMana%20Generation%20Toggle false)
        (Variables|Cast|SetCast%20Time _returnvalue)
        (Variables|Cast|SetMax%20Cast%20Time _returnvalue)
        (Variables|Cast|SetCast true)
        (Development|PrintString (Utilities|String|Append (Utilities|String|Append (Utilities|String|Append (Utilities|String|Append "Casting: " (Utilities|String|ToString(Name) (.name _item))) " in ") (Utilities|String|ToString(Float) _returnvalue)) "sec"))
        (else
          (Development|PrintString "Unable to Cast")))
      (else
        (Development|PrintString "Need more health!")))
    (elif (>= (Variables|Default|GetCurrent%20Mana) (.mana _item))
      (goto _label)
      (else
        (Development|PrintString "Need more mana")))))

(event Custom|Spell%20Trigger
  (bind _returnvalue (Components|GetOwner))
  (bind _spell_list (Variables|Default|GetSpell%20List))
  (bind _selected_spell (Variables|Default|GetSelected%20Spell))
  (bind _item (Utilities|Array|Get(acopy) _spell_list _selected_spell))
  ;[1 1 1] Spell Triggerd
  (CallFunction|CheckStock)
  (if (.blood_magic _item)
    (Variables|Default|SetCurrent%20Life (- (Variables|Default|GetCurrent%20Life) (.mana _item)))
    (else
      (Variables|Default|SetCurrent%20Mana (- (Variables|Default|GetCurrent%20Mana) (.mana _item)))))
  (bind _returnvalue_2 (Game|SpawnActorfromClass (.magic_bp _item) (Math|Conversions|ToTransform(Vector) (Transformation|GetActorLocation (Components|GetOwner))) false 0))
  (Development|PrintString (Utilities|GetDisplayName _returnvalue))
  (Variables|/Game/Blueprint/Component/Spell.Spell_C|SetPower (Utilities|Array|Get(acopy) (Actor|GetComponentsByClass _returnvalue_2 "/Game/Blueprint/Component/Spell.Spell_C")) (.power _item))
  (Variables|/Game/Blueprint/Component/Spell.Spell_C|SetActor%20Owner (Utilities|Array|Get(acopy) (Actor|GetComponentsByClass _returnvalue_2 "/Game/Blueprint/Component/Spell.Spell_C")) _returnvalue)
  (Variables|/Game/Blueprint/Component/Spell.Spell_C|SetLife%20Span (Utilities|Array|Get(acopy) (Actor|GetComponentsByClass _returnvalue_2 "/Game/Blueprint/Component/Spell.Spell_C")) (.lifespan _item))
  (CallFunction|SetCooldown (.cooldown _item) (Variables|Default|GetSelected%20Spell))
  (Variables|Default|SetGlobal%20Cooldown 0.5))

(event Custom|Set%20Target%20Type
  ;[1 1 1] Decals
  (switch Utilities|FlowControl|Switch|Switchonenum_magic_target "NewEnumerator2"))

(event Custom|Channel
  ;[1 1 1] Channel
  (if (.channel (Utilities|Array|Get(acopy) (Variables|Default|GetSpell%20List) (Variables|Default|GetSelected%20Spell)))
    _))

(event Custom|Action%20Release
  (params (Action :type Integer :default 0))
  ;[1 1 1] Check Button Up and run selected attack
  (Variables|Default|SetSelected%20Spell Action)
  (CallFunction|SetCastTimer)
  (Variables|Default|SetDown false))

(event Custom|Action%20Press
  (params (Action :type Integer :default 0))
  ;[1 1 1] Check Button Down and charge selected attack
  (Variables|Default|SetSelected%20Spell Action)
  (CallFunction|Channel)
  (Variables|Default|SetShow%20Decal true)
  (Variables|Default|SetDown true))

(event EventTick
  (params (DeltaSeconds :type Float%20%28single-precision%29))
  (bind _returnvalue (Components|GetOwner))
  (bind _returnvalue_2 (Transformation|GetVelocity _returnvalue))
  (CallFunction|SetMax)
  (if (Variables|Default|GetShow%20Decal)
    (CallFunction|SetTargetType))
  (CallFunction|Generation DeltaSeconds)
  (CallFunction|Cooldown DeltaSeconds)
  ;[1 1 1] Cast Timer
  (if (Math|Boolean|ANDBoolean (Variables|Cast|GetCast) (Math|Float|NearlyEqual(Float) (+ (.x _returnvalue_2) (.y _returnvalue_2) (.z _returnvalue_2)) 0.0 (.focus (.secondary (Variables|Default|GetStats)))) (>= (Variables|Cast|GetMax%20Cast%20Time) 0.0))
    (bind _output_get (Variables|Cast|SetCast%20Time (- (Variables|Cast|GetCast%20Time) DeltaSeconds)))
    (if (<= _output_get 0.0) ; If cast time is zero, trigger spell
      (Variables|Cast|SetMax%20Cast%20Time -0.1)
      (CallFunction|SpellTrigger))
    (else
      (Variables|Cast|SetMax%20Cast%20Time -0.1)
      (Variables|Cast|SetCast false)
      (Variables|Default|SetMana%20Generation%20Toggle true)
      (if (not (Variables|Default|GetDown))
        (Variables|Default|SetShow%20Decal false)))))

(event EventInitializeComponent
  ;[1 1 1] Init
  (CallFunction|Setup))

(fn Cooldown
  (params (delta :type Float%20%28single-precision%29))
  (for (_array_element _array_index) (Variables|Default|GetSpell%20List)
    (bind _output_get (LocalVariables|SetStock (.Stock_Current (Utilities|Struct|BreakSpellStruct2 _array_element))))
    (if (>= (.current_cooldown (Utilities|Struct|BreakSpellStruct2 _array_element)) 0.0)
      (LocalVariables|Setcd (- (.current_cooldown (Utilities|Struct|BreakSpellStruct2 _array_element)) delta) :!label _label)
      (elif (and (> (.Stock_Max (Utilities|Struct|BreakSpellStruct2 _array_element)) 0) (> (.Stock_Max (Utilities|Struct|BreakSpellStruct2 _array_element)) _output_get))
        (LocalVariables|SetStock (+ _output_get 1))
        (LocalVariables|Setcd (.Cooldown (Utilities|Struct|BreakSpellStruct2 _array_element)))
        (else
          (goto _label))))
    (Utilities|Array|SetArrayElem (Variables|Default|GetSpell%20List) _array_index (Utilities|Struct|MakeSpellStruct2 (.Name (Utilities|Struct|BreakSpellStruct2 _array_element)) (.Description (Utilities|Struct|BreakSpellStruct2 _array_element)) (.Icon (Utilities|Struct|BreakSpellStruct2 _array_element)) (.Power (Utilities|Struct|BreakSpellStruct2 _array_element)) (.Mana (Utilities|Struct|BreakSpellStruct2 _array_element)) (.Blood_Magic (Utilities|Struct|BreakSpellStruct2 _array_element)) (.CastTime (Utilities|Struct|BreakSpellStruct2 _array_element)) (.Cooldown (Utilities|Struct|BreakSpellStruct2 _array_element)) (LocalVariables|Getcd) (.Spell_ParticleBP (Utilities|Struct|BreakSpellStruct2 _array_element)) (.Magic_BP (Utilities|Struct|BreakSpellStruct2 _array_element)) (.Animation (Utilities|Struct|BreakSpellStruct2 _array_element)) (.LifeSpan (Utilities|Struct|BreakSpellStruct2 _array_element)) (.Channel (Utilities|Struct|BreakSpellStruct2 _array_element)) (.Area_Of_Effect (Utilities|Struct|BreakSpellStruct2 _array_element)) (.Area_of_Effect_Size (Utilities|Struct|BreakSpellStruct2 _array_element)) (.Stock_Max (Utilities|Struct|BreakSpellStruct2 _array_element)) (LocalVariables|GetStock))))
  (if (> (Variables|Default|GetGlobal%20Cooldown) 0.0)
    (Variables|Default|SetGlobal%20Cooldown (- (Variables|Default|GetGlobal%20Cooldown) delta))))

(fn SetCooldown
  (params (cooldown :type Float%20%28single-precision%29 :default 0.0) (id :type Integer :default 0))
  (bind _spell_list (Variables|Default|GetSpell%20List))
  (bind _item (Utilities|Array|Get(acopy) _spell_list id))
  (bind (_name _description _icon _power _mana _blood_magic _casttime _cooldown _current_cooldown _spell_particlebp _magic_bp _animation _lifespan _channel _area_of_effect _area_of_effect_size _stock_max _stock_current) (Utilities|Struct|BreakSpellStruct2 _item))
  (if (not (> _stock_max 0))
    (Utilities|Array|SetArrayElem _spell_list id (Utilities|Struct|MakeSpellStruct2 _name _description _icon _power _mana _blood_magic _casttime _cooldown cooldown _spell_particlebp _magic_bp _animation _lifespan _channel _area_of_effect _area_of_effect_size _stock_max _stock_current))))

(fn CheckStock
  (bind _spell_list (Variables|Default|GetSpell%20List))
  (bind _selected_spell (Variables|Default|GetSelected%20Spell))
  (bind _item (Utilities|Array|Get(acopy) _spell_list _selected_spell))
  (bind (_name _description _icon _power _mana _blood_magic _casttime _cooldown _current_cooldown _spell_particlebp _magic_bp _animation _lifespan _channel _area_of_effect _area_of_effect_size _stock_max _stock_current) (Utilities|Struct|BreakSpellStruct2 _item))
  (if (and (> _stock_current 0) (> _stock_max 0))
    (LocalVariables|SetStock (- _stock_current 1)))
  (Utilities|Array|SetArrayElem _spell_list _selected_spell (Utilities|Struct|MakeSpellStruct2 _name _description _icon _power _mana _blood_magic _casttime _cooldown _current_cooldown _spell_particlebp _magic_bp _animation _lifespan _channel _area_of_effect _area_of_effect_size _stock_max (LocalVariables|GetStock))))